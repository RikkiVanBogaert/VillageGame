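; BP_HousePlacer is a mouse-driven placement actor that spawns a BP_House at the clicked world location.
; On BeginPlay it enables input, makes itself the player's view target and shows the cursor.
; PlaceHouse turns on placement mode, during which Tick line-traces from the cursor along the Visibility channel with debug drawing.
; A left click on a valid hit spawns the house there and ends placement mode.
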(event `self.ReceiveBeginPlay`
  (bind _returnvalue (`GameplayStatics.GetPlayerController` 0))
  (`self.EnableInput` _returnvalue)
  (`PlayerController.SetViewTargetWithBlend` _returnvalue self 0.0 "VTBlend_Linear" 0.0 false)
  (set `PlayerController.bShowMouseCursor` true _returnvalue))

(event `self.ReceiveTick`
  (params (DeltaSeconds :type "Float (single-precision)"))
  (bind (_worldlocation _worlddirection) (`PlayerController.DeprojectMousePositionToWorld` (`GameplayStatics.GetPlayerController` 0)))
  (if (`self.placingHouse`)
    (bind (_outhit _returnvalue) (`KismetSystemLibrary.LineTraceSingle` :`Start` _worldlocation :`End` (+ _worldlocation (* _worlddirection 10000.0)) :`TraceChannel` "TraceTypeQuery1" :`DrawDebugType` "ForOneFrame"))))

(event `Key|LeftMouseButton`
  (params (Key :type "Key Structure"))
  (:`Pressed`
    (if (stale `self.ReceiveTick` _returnvalue)
      (if (`self.placingHouse`)
        (`|SpawnActorFromClass` "/Game/Blueprints/BP_House.BP_House_C" (`KismetMathLibrary.MakeTransform` (`.Location` (`GameplayStatics.BreakHitResult` (stale `self.ReceiveTick` _outhit)))) "Undefined" "MultiplyWithRoot" null null)
        (set `self.placingHouse` false)))))

(fn `PlaceHouse`
  (set `self.placingHouse` true))

(fn `UserConstructionScript`)
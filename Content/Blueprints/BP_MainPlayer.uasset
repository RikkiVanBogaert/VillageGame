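; Player pawn that moves the camera and places houses on grid cells with the mouse.
; BeginPlay adds the Enhanced Input context and shows the cursor; movement input is applied relative to control rotation.
; PlaceHouse arms placement, making Tick line-trace under the cursor with debug drawing.
; Left click places a house on the traced BP_GridCell if it is unoccupied, then disarms placement.
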(event `self.ReceiveBeginPlay`
  (bind _returnvalue (`GameplayStatics.GetPlayerController` 0))
  ;[1 1 1] Handle Input
  (bind _asbp_my_controller (cast `/Game/Blueprints/BP_MyController` (`GameplayStatics.GetPlayerController` 0)))
  (`EnhancedInputSubsystemInterface.AddMappingContext` (pcsubsystem `EnhancedInputLocalPlayerSubsystem` _asbp_my_controller) "/Game/Input/InputMap.InputMap" 0 (struct))
  ;;[1 1 1] Show mouse for placing house
  (`self.EnableInput` _returnvalue)
  (`PlayerController.SetViewTargetWithBlend` _returnvalue self 0.0 "VTBlend_Linear" 0.0 false)
  (set `PlayerController.bShowMouseCursor` true _returnvalue))

(event `EnhancedInput|/Game/Input/Movement`
  (params (ActionValue :type "Vector2D Structure") (ElapsedSeconds :type "Float (double-precision)") (TriggeredSeconds :type "Float (double-precision)") (InputAction :type "InputAction Object Reference" :default "/Game/Input/Movement.Movement"))
  ;[1 1 1] Handle Input
  (:`Triggered`
    (`self.MoveCamera` ActionValue_X ActionValue_Y)))

(event `self.ReceiveTick`
  (params (DeltaSeconds :type "Float (single-precision)"))
  (bind (_worldlocation _worlddirection) (`PlayerController.DeprojectMousePositionToWorld` (`GameplayStatics.GetPlayerController` 0)))
  ;[1 1 1] Place House
  (if (`self.canPlaceHouse`)
    (bind _outhit (`KismetSystemLibrary.LineTraceSingle` :`Start` _worldlocation :`End` (+ _worldlocation (* _worlddirection 10000.0)) :`TraceChannel` "TraceTypeQuery1" :`DrawDebugType` "ForOneFrame"))))

(event `Key|LeftMouseButton`
  (params (Key :type "Key Structure"))
  ;[1 1 1] Place House
  (:`Pressed`
    (bind _asbp_grid_cell (cast `/Game/Blueprints/Assets/BP_GridCell` (`.HitActor` (`GameplayStatics.BreakHitResult` (stale `self.ReceiveTick` _outhit)))))
    (if (`/Game/Blueprints/Assets/BP_GridCell.isOccupied` _asbp_grid_cell)
      _
      (elif (`self.canPlaceHouse`)
        (`/Game/Blueprints/Assets/BP_GridCell.PlaceHouse` _asbp_grid_cell)
        (set `self.canPlaceHouse` false)))))

(fn `MoveCamera`
  (params (X :type "Float (single-precision)") (Y :type "Float (double-precision)"))
  (bind (_returnvalue_roll _returnvalue_pitch _returnvalue_yaw) (`KismetMathLibrary.BreakRotator` (`self.GetControlRotation`)))
  (bind (_returnvalue_roll_2 _returnvalue_pitch_2 _returnvalue_yaw_2) (`KismetMathLibrary.BreakRotator` (`self.GetControlRotation`)))
  (`self.AddMovementInput` (`KismetMathLibrary.GetForwardVector` (`KismetMathLibrary.MakeRotator` 0.0 0.0 _returnvalue_yaw)) X)
  (`self.AddMovementInput` (`KismetMathLibrary.GetRightVector` (`KismetMathLibrary.MakeRotator` _returnvalue_roll_2 0.0 _returnvalue_yaw_2)) Y))

(fn `PlaceHouse`
  (set `self.canPlaceHouse` true))

(fn `UserConstructionScript`)
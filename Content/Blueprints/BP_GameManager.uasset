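; BP_GameManager is an actor that tracks the game state and runs a timed Preparation phase before play begins.
; Tick switches on GameState and, during Preparation, calls CalculatePrepTime to accumulate delta time in Timer.
; When Timer reaches PrepTime, the state changes to Playing and a "PLAY!" message prints; no other state has logic yet.
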(event `self.ReceiveTick`
  (params (DeltaSeconds :type "Float (single-precision)"))
  (switch `/Game/Blueprints/Enum_GameStates` (`self.gameState`)
    (:`NewEnumerator0`
      (`self.CalculatePrepTime` DeltaSeconds))))

(fn `CalculatePrepTime`
  (params (deltaSeconds :type "Float (double-precision)"))
  (bind _output_get (set `self.timer` (+ (`self.timer`) deltaSeconds)))
  (if (>= _output_get (`self.prepTime`))
    (set `self.gameState` "NewEnumerator1")
    (`KismetSystemLibrary.PrintString` "PLAY!")))

(fn `UserConstructionScript`)
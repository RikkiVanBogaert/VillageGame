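; BP_MyPawn is the player pawn, combining Enhanced Input movement with click-to-place house building.
; BeginPlay adds the input mapping context through BP_MyController, sets the view to the pawn and shows the cursor.
; PlaceHouse enables placement mode, during which Tick line-traces from the mouse cursor into the world with debug drawing.
; A left click on BP_HomeGround spawns BP_House at the hit location and ends placement mode.
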(event `self.ReceiveBeginPlay`
  (bind _returnvalue (`GameplayStatics.GetPlayerController` 0))
  ;[1 1 1] Handle Input
  (bind _asbp_my_controller (cast `/Game/Blueprints/BP_MyController` (`GameplayStatics.GetPlayerController` 0)))
  (`EnhancedInputSubsystemInterface.AddMappingContext` (pcsubsystem `EnhancedInputLocalPlayerSubsystem` _asbp_my_controller) "/Game/Input/InputMap.InputMap" 0 (struct))
  ;;[1 1 1] Show mouse for placing house
  (`self.EnableInput` _returnvalue)
  (`PlayerController.SetViewTargetWithBlend` _returnvalue self 0.0 "VTBlend_Linear" 0.0 false)
  (set `PlayerController.bShowMouseCursor` true _returnvalue))

(event `EnhancedInput|/Game/Input/Movement`
  (params (ActionValue :type "Vector2D Structure") (ElapsedSeconds :type "Float (double-precision)") (TriggeredSeconds :type "Float (double-precision)") (InputAction :type "InputAction Object Reference" :default "/Game/Input/Movement.Movement"))
  (bind (_returnvalue_roll _returnvalue_pitch _returnvalue_yaw) (`KismetMathLibrary.BreakRotator` (`self.GetControlRotation`)))
  (bind (_returnvalue_roll_2 _returnvalue_pitch_2 _returnvalue_yaw_2) (`KismetMathLibrary.BreakRotator` (`self.GetControlRotation`)))
  ;[1 1 1] Handle Input
  (:`Triggered`
    (`self.AddMovementInput` (`KismetMathLibrary.GetForwardVector` (`KismetMathLibrary.MakeRotator` 0.0 0.0 _returnvalue_yaw)) ActionValue_X)
    (`self.AddMovementInput` (`KismetMathLibrary.GetRightVector` (`KismetMathLibrary.MakeRotator` _returnvalue_roll_2 0.0 _returnvalue_yaw_2)) ActionValue_Y)))

(event `self.ReceiveTick`
  (params (DeltaSeconds :type "Float (single-precision)"))
  (bind (_worldlocation _worlddirection) (`PlayerController.DeprojectMousePositionToWorld` (`GameplayStatics.GetPlayerController` 0)))
  ;[1 1 1] Place House
  (if (`self.IsPlacingHouse`)
    (bind (_outhit _returnvalue) (`KismetSystemLibrary.LineTraceSingle` :`Start` _worldlocation :`End` (+ _worldlocation (* _worlddirection 10000.0)) :`TraceChannel` "TraceTypeQuery1" :`DrawDebugType` "ForOneFrame"))))

(event `Key|LeftMouseButton`
  (params (Key :type "Key Structure"))
  ;[1 1 1] Place House
  (:`Pressed`
    (bind (_bblockinghit _binitialoverlap _time _distance _location _impactpoint _normal _impactnormal _physmat _hitactor) (`GameplayStatics.BreakHitResult` (stale `self.ReceiveTick` _outhit)))
    (if (== (`GameplayStatics.GetObjectClass` _hitactor) "/Game/Blueprints/BP_HomeGround.BP_HomeGround_C")
      (if (stale `self.ReceiveTick` _returnvalue)
        (if (`self.IsPlacingHouse`)
          (`|SpawnActorFromClass` "/Game/Blueprints/BP_House.BP_House_C" (`KismetMathLibrary.MakeTransform` _location) "Undefined" "MultiplyWithRoot" null null)
          (set `self.IsPlacingHouse` false))))))

(fn `PlaceHouse`
  (set `self.IsPlacingHouse` true))

(fn `UserConstructionScript`)
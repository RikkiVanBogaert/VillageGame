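; BP_HomeGround is a ground actor that spawns a three-by-three grid of BP_GridCell actors on BeginPlay.
; CreateGrid uses the Plane component as the template, taking its world location as the start, its mesh bounds for cell size and its world scale for each cell.
; IncrementX, IncrementY and ResetX move the spawn position, stepping by scaled size plus Offset and wrapping to a new row after every third cell.
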(event `self.ReceiveBeginPlay`
  (`self.CreateGrid`))

(fn `CreateGrid`
  (bind _plane (`self.Plane`))
  (bind (_returnvalue_min _returnvalue_max) (break `Box` (`StaticMesh.GetBoundingBox` (`StaticMeshComponent.StaticMesh` _plane))))
  (set `self.cellTransform` (`SceneComponent.K2_GetComponentLocation` _plane))
  (set `self.sizeBox` (- _returnvalue_max _returnvalue_min))
  (for _index (range 1 10)
    (`|SpawnActorFromClass` "/Game/Blueprints/Assets/BP_GridCell.BP_GridCell_C" (`KismetMathLibrary.MakeTransform` (`self.cellTransform`) (struct) (`SceneComponent.K2_GetComponentScale` _plane)) "Undefined" "MultiplyWithRoot" null null)
    (`self.IncrementX`)
    (if (== (mod _index 3) 0)
      (`self.IncrementY`)
      (`self.ResetX`))))

(fn `IncrementX`
  (bind _sizebox_x (`KismetMathLibrary.BreakVector` (`self.sizeBox`)))
  (bind (_celltransform_x _celltransform_y _celltransform_z) (`KismetMathLibrary.BreakVector` (`self.cellTransform`)))
  (bind _returnvalue_x (`KismetMathLibrary.BreakVector` (`SceneComponent.K2_GetComponentScale` (`self.Plane`))))
  (set `self.cellTransform` (`KismetMathLibrary.MakeVector` (+ (+ _celltransform_x (* _sizebox_x _returnvalue_x)) (`self.offset`)) _celltransform_y _celltransform_z)))

(fn `IncrementY`
  (bind (_sizebox_x _sizebox_y) (`KismetMathLibrary.BreakVector` (`self.sizeBox`)))
  (bind (_celltransform_x _celltransform_y _celltransform_z) (`KismetMathLibrary.BreakVector` (`self.cellTransform`)))
  (bind (_returnvalue_x _returnvalue_y) (`KismetMathLibrary.BreakVector` (`SceneComponent.K2_GetComponentScale` (`self.Plane`))))
  (set `self.cellTransform` (`KismetMathLibrary.MakeVector` _celltransform_x (+ (+ _celltransform_y (* _sizebox_y _returnvalue_y)) (`self.offset`)) _celltransform_z)))

(fn `ResetX`
  (bind (_celltransform_x _celltransform_y _celltransform_z) (`KismetMathLibrary.BreakVector` (`self.cellTransform`)))
  (bind _returnvalue_x (`KismetMathLibrary.BreakVector` (`SceneComponent.K2_GetComponentLocation` (`self.Plane`))))
  (set `self.cellTransform` (`KismetMathLibrary.MakeVector` _returnvalue_x _celltransform_y _celltransform_z)))

(fn `UserConstructionScript`)
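; BP_House is a spawner building that produces BP_Attacker AI pawns during play.
; On BeginPlay it caches the BP_GameManager, and each Tick it advances a timer only while that manager's GameState is Playing.
; When the timer reaches CharSpawnInterval, it spawns an attacker at the SpawnPoint component's location, prints a debug string and resets the timer.
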(event `self.ReceiveBeginPlay`
  (bind _returnvalue (`GameplayStatics.GetActorOfClass` "/Game/Blueprints/BP_GameManager.BP_GameManager_C"))
  (set `self.gameManager` _returnvalue))

(event `self.ReceiveTick`
  (params (DeltaSeconds :type "Float (single-precision)"))
  (switch `/Game/Blueprints/Enum_GameStates` (`/Game/Blueprints/BP_GameManager.gameState` (`self.gameManager`))
    (:`NewEnumerator1`
      (`self.SpawnAttackerOnTimeInterval` DeltaSeconds))))

(fn `SpawnAttacker`
  (`KismetSystemLibrary.PrintString` "Spawn Attacker" true true (struct :`G` 0.66 :`B` 1.0 :`A` 1.0) 10.0)
  (`AIBlueprintHelperLibrary.SpawnAIFromClass` "/Game/Blueprints/Assets/BP_Attacker.BP_Attacker_C" null (`SceneComponent.K2_GetComponentLocation` (`self.SpawnPoint`)) (struct) false null))

(fn `SpawnAttackerOnTimeInterval`
  (params (deltaSeconds :type "Float (double-precision)"))
  (bind _output_get (set `self.timer` (+ (`self.timer`) deltaSeconds)))
  (if (>= _output_get (`self.charSpawnInterval`))
    (`self.SpawnAttacker`)
    (set `self.timer` 0.0)))

(fn `UserConstructionScript`)
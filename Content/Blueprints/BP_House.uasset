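; House actor that periodically spawns BP_Attacker AI pawns while the game is running.
; A looping timer started on BeginPlay fires SpawnCharacter, which looks up the BP_GameInfo actor and skips spawning once IsGameOver is set.
; SpawnAttacker creates the pawn at the SpawnPoint component's world location and prints a debug message.
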(event `self.ReceiveBeginPlay`
  (`KismetSystemLibrary.K2_SetTimerDelegate` (delegate `Event Spawn Character`) 4.0 true))

(event `Event Spawn Character`
  (bind _returnvalue (`GameplayStatics.GetActorOfClass` "/Game/Blueprints/BP_GameInfo.BP_GameInfo_C"))
  (if (not (`/Game/Blueprints/BP_GameInfo.isGameOver` _returnvalue))
    (`self.SpawnAttacker`)))

(fn `SpawnAttacker`
  (`KismetSystemLibrary.PrintString` "Spawn Attacker" true true (struct :`G` 0.66 :`B` 1.0 :`A` 1.0) 10.0)
  (`AIBlueprintHelperLibrary.SpawnAIFromClass` "/Game/Blueprints/BP_Attacker.BP_Attacker_C" null (`SceneComponent.K2_GetComponentLocation` (`self.SpawnPoint`)) (struct) false null))

(fn `UserConstructionScript`)